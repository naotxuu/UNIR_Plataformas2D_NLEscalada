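; BP_Bullet is a projectile actor for the 2D platformer weapons.
; Every tick it moves along its forward vector at Speed, scaled by delta time, using a non-swept location set rather than a movement component.
; A timer started on BeginPlay destroys it after a short lifetime, and the overlap event is empty, so it applies no hit logic.
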(event `self.ReceiveBeginPlay`
  (`KismetSystemLibrary.K2_SetTimerDelegate` (delegate `DestroyBullet`) 3.0))

(event `DestroyBullet`
  (`self.K2_DestroyActor`))

(event `self.ReceiveActorBeginOverlap`
  (params (OtherActor :type "Actor Object Reference")))

(event `self.ReceiveTick`
  (params (DeltaSeconds :type "Float (single-precision)"))
  (`self.K2_SetActorLocation` (+ (`self.K2_GetActorLocation`) (* (* (`self.speed`) DeltaSeconds) (`self.GetActorForwardVector`)))))

(fn `UserConstructionScript`)